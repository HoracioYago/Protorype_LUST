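; BP_Gates is a double gate actor that swings two leaves open and closed when its Gate event is called.
; Gate runs a FlipFlop that alternately plays and reverses the opening timeline.
; On each update, the timeline value scaled by DoorAngle yaws the Arrow and Arrow1 pivots in opposite directions.
; A debug "Start" string prints on every call.
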(event Custom|Gate
  (Development|PrintString "Start")
  (Utilities|FlowControl|FlipFlop
    (:A
      (bind _newtrack_0 (Timeline|Timeline_opening Play)
        (:Update
          (Transformation|SetRelativeRotation (Variables|Default|GetArrow) (Math|Rotator|MakeRotator 0.0 0.0 (* _newtrack_0 (* (Variables|Default|GetDoor%20Angle) -1.0))) false false)
          (Transformation|SetRelativeRotation (Variables|Default|GetArrow1) (Math|Rotator|MakeRotator 0.0 0.0 (* _newtrack_0 (Variables|Default|GetDoor%20Angle))) false false))))
    (:B
      (Timeline|Timeline_opening Reverse))))

(event EventBeginPlay)

(event Collision|EventActorBeginOverlap
  (params (OtherActor :type Actor%20Object%20Reference)))

(event EventTick
  (params (DeltaSeconds :type Float%20%28single-precision%29)))

(fn ConstructionScript)