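; Player character for a top-down-style game that turns its Cube component toward the mouse cursor and tracks score, death and save state.
; Each Tick it deprojects the cursor and intersects a camera line with a horizontal plane at actor height to aim the Cube.
; BeginPlay adds the score HUD and restores transform and score from the GameInstance message, skipping default-transform saves.
; Helper functions toggle a widget panel, show the death screen and build save data.
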(event EventBeginPlay
  (bind _returnvalue (UserInterface|CreateWidget "/Game/Omid/UI/WBP_Score.WBP_Score_C"))
  (UserInterface|Viewport|AddtoViewport _returnvalue 0)
  (bind _savegamedata (Class|BPISaveGame|GetGameData(Message) (Game|GetGameInstance)))
  (Utilities|IsValid _savegamedata
    (:Is%20Valid
      (CallFunction|UsePlayerSave (Variables|/Game/real/SaveSystem/SG_Demo.SG_Demo_C|GetPlayerSave _savegamedata)))))

(event EventTick
  (params (DeltaSeconds :type Float%20%28single-precision%29))
  (bind _returnvalue (Game|GetPlayerController 0))
  (bind _returnvalue_2 (Transformation|GetActorLocation))
  (bind (_worldlocation _worlddirection) (Game|Player|ConvertMouseLocationToWorldSpace _returnvalue))
  (Transformation|SetWorldRotation (Variables|Default|GetCube) (Math|Rotator|FindLookatRotation _returnvalue_2 (.Intersection (Class|KismetMathLibrary|LinePlaneIntersectionOriginNormal (Transformation|GetActorLocation (Game|GetPlayerCameraManager 0)) (+ _worldlocation (* _worlddirection 5e+03)) _returnvalue_2 "0.000000,0.000000,1.000000"))) false false))

(fn ConstructionScript)

(fn ToggleUI
  (params (ShouldShow :type Boolean))
  (bind _widget (Variables|Default|GetWidget))
  (bind _canvaspanel_26 (Variables|/Game/Omid/UI/WB_Interface.WB_Interface_C|GetCanvasPanel_26 _widget))
  (if ShouldShow
    (Widget|SetVisibility _canvaspanel_26 "Visible")
    (Variables|UI|SetIsUIVisible true)
    (else
      (Widget|SetVisibility _canvaspanel_26 "Hidden")
      (Variables|UI|SetIsUIVisible false))))

(fn ShowDeathScreen
  (Variables|UI|SetIsPlayerDead true)
  (bind _returnvalue (UserInterface|CreateWidget "/Game/Omid/UI/WB_DeathScreen.WB_DeathScreen_C"))
  (UserInterface|Viewport|AddtoViewport _returnvalue 0))

(fn GetPlayerSave
  (return (Utilities|Struct|MakeS_PlayerSave false (Variables|UI|GetScore) (Transformation|GetActorTransform))))

(fn UsePlayerSave
  (params (PlayerSave :type S%20Player%20Save%20Structure))
  (if (not (== (.playertransform PlayerSave) (Math|Transform|MakeTransform "0, 0, 0")))
    (Transformation|SetActorTransform (.playertransform PlayerSave))
    (Variables|UI|SetScore (.score PlayerSave))))