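; Machine gun enemy that sweeps its yaw between limits as a searchlight and turns to track tagged targets; no firing logic here.
; While Active, Tick line-traces forward to set Alert, then either snaps yaw toward the hit actor or runs the patrol sweep.
; The sweep uses a timeline with pauses at each reversal, noted as frame-rate dependent.
; A retriggerable delay clears Alert after sight is lost.
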(event Custom|TrackPlayer
  (if (Variables|Status|GetAlert)
    (Transformation|SetActorRotation (Math|Rotator|MakeRotator 0.0 0.0 (.yaw (Math|Rotator|FindLookatRotation (Transformation|GetActorLocation) (Transformation|GetActorLocation (.HitActor (Collision|BreakHitResult (Variables|Detection|GetHitResult)))))))) ; follow player pawn
  ))

(event Custom|SwitchDirection
  ;[1 1 1] EnemyRotation
  (Variables|Sweep|SetStopped true)
  (Utilities|FlowControl|Delay (Variables|Sweep|GetPauseDuration))
  (Utilities|FlowControl|FlipFlop
    (:A
      (Variables|Sweep|SetSwitchRotation false)
      (Variables|Sweep|SetStopped false))
    (:B
      (Variables|Sweep|SetSwitchRotation true)
      (Variables|Sweep|SetStopped false)))
  (CallFunction|RotationMov))

(event Custom|ExitAlertTimer
  (if (Variables|Status|GetAlert)
    (if (Variables|Detection|GetOnSight)
      (Utilities|FlowControl|RetriggerableDelay (Variables|Detection|GetAlertDuration) :!label _label)
      (if (Variables|Detection|GetOnSight)
        (Variables|Status|SetAlert true)
        (goto _label)
        (else
          (Variables|Status|SetAlert false)
          (Variables|Status|SetPatrol true))))))

(event Custom|RotationMov
  ;[1 1 1] Raycast & Rotation (Frame rate ruins it HAVE TO FIX)
  (if (not (Variables|Status|GetAlert))
    (if (Variables|Sweep|GetStopped)
      (bind (_direction _add_rotation _subrotation) (Timeline|Rotation%20animation Stop)
        (:Update
          (if (Variables|Sweep|GetSwitchRotation)
            (Class|Actor|AddActorWorldRotation (Math|Rotator|MakeRotator 0.0 0.0 (* (Variables|Sweep|GetRotationSpeed) _add_rotation)))
            (else
              (Class|Actor|AddActorWorldRotation (Math|Rotator|MakeRotator 0.0 0.0 (* _subrotation (Variables|Sweep|GetRotationSpeed))))))
          (Transformation|SetActorRotation (Math|Rotator|MakeRotator 0.0 0.0 (Math|Float|Clamp(Float) (.yaw (Transformation|GetActorRotation)) (Variables|Sweep|GetMinLimit) (Variables|Sweep|GetMaxLimit)))))
        (:Finished
          (CallFunction|SwitchDirection)))
      (elif (Variables|Sweep|GetSwitchRotation)
        (Timeline|Rotation%20animation Play)
        (else
          (Timeline|Rotation%20animation Reverse))))))

(event EventBeginPlay
  ;[1 1 1] EnemyRotation
  (if (Variables|Status|GetPatrol)
    (CallFunction|RotationMov)
    (Components|Timeline|SetPlayRate (Variables|Default|GetRotation%20animation) (/ 1.0 (Variables|Sweep|GetSweepRate)))))

(event EventTick
  (params (DeltaSeconds :type Float%20%28single-precision%29))
  ;[1 1 1] Raycast Searchlight
  (if (Variables|Status|GetActive)
    (CallFunction|Search)
    (if (Variables|Status|GetAlert)
      (CallFunction|TrackPlayer)
      (CallFunction|ExitAlertTimer)
      (else
        (CallFunction|RotationMov)))))

(fn ConstructionScript
  (if (Variables|FieldOfVision|Debug|GetbRebuild)
    _
    (else
      _))
  (bind _output_get (Variables|FieldOfVision|Auxiliary|SetNumberOfSections (Math|Float|Ceil (/ (* 0.0 2.0) 0.0))))
  (Variables|FieldOfVision|Auxiliary|SetdAngle (/ (* 0.0 2.0) _output_get))
  (for _index (range 0 (Variables|FieldOfVision|Auxiliary|GetNumberOfSections))
    _))

(fn Search
  ;[1 1 1] Searchlight Logic
  (CallFunction|Start)
  (CallFunction|LineTracing))

(fn Start
  ;[1 1 1] Create Raycast Parameters
  (if (Variables|FieldOfVision|Debug|GetbRebuild)
    (Variables|FieldOfVision|Auxiliary|SetStartPoint (+ (Math|Vector|MakeVector 0.0 0.0 (- (Variables|FieldOfVision|Base|GetHeightOfCheck) 1e+02)) (Transformation|GetActorLocation)))
    (return)))

(fn LineTracing
  (bind _startpoint (Variables|FieldOfVision|Auxiliary|GetStartPoint))
  ;[1 1 1] Raycast
  (bind (_outhit _returnvalue) (Collision|LineTraceByChannel _startpoint (+ _startpoint (* (Transformation|GetActorForwardVector) (Variables|FieldOfVision|Base|GetSightRange))) "TraceTypeQuery1" false 0 "ForOneFrame"))
  (if _returnvalue
    (if (Actor|ActorHasTag (.HitActor (Collision|BreakHitResult _outhit)) (Variables|Detection|GetDetectablePawnTag))
      (Variables|Detection|SetHitResult _outhit)
      (Variables|Detection|SetOnSight true)
      (Development|PrintString "I SEE YOU!" false)
      (Variables|Status|SetAlert true)
      (Variables|Detection|SetAlertDuration 5.0)
      (else
        (Variables|Detection|SetOnSight false)))))