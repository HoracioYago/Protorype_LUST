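; PC_Example is a player controller Blueprint that drives BP_Character through Enhanced Input with a visible mouse cursor.
; BeginPlay caches the pawn and adds MC_Example; IA_Move moves it along its forward and right vectors unless aiming.
; IA_Aim sets the aiming flag and draws a forward debug trace whose result is unused, while IA_Pull only prints.
; Cursor-facing rotation via line-plane intersection exists but is disconnected.
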(event Input|EnhancedActionEvents|EnhancedInputActionIA_Pull
  (params (ActionValue :type Boolean) (ElapsedSeconds :type Float%20%28double-precision%29) (TriggeredSeconds :type Float%20%28double-precision%29) (InputAction :type Input%20Action%20Object%20Reference :default "/Game/real/Inputs/IA_Pull.IA_Pull"))
  (if (Variables|Default|GetAiming)
    (Development|PrintString "Pull")))

(event Input|EnhancedActionEvents|EnhancedInputActionIA_Move
  (params (ActionValue :type Vector%202D%20Structure) (ElapsedSeconds :type Float%20%28double-precision%29) (TriggeredSeconds :type Float%20%28double-precision%29) (InputAction :type Input%20Action%20Object%20Reference :default "/Game/real/Inputs/IA_Move.IA_Move"))
  (bind (_x _y) (Math|Vector2D|BreakVector2D ActionValue))
  (bind _as_bp_character (Variables|Default|GetAs%20BP%20Character))
  (bind _as_bp_character_2 (Variables|Default|GetAs%20BP%20Character))
  (if (not (Variables|Default|GetAiming))
    (Pawn|Input|AddMovementInput _as_bp_character_2 (Transformation|GetActorForwardVector _as_bp_character_2) _x false)
    (Pawn|Input|AddMovementInput _as_bp_character (Transformation|GetActorRightVector _as_bp_character) _y false)))

(event Input|EnhancedActionEvents|EnhancedInputActionIA_Aim
  (params (ActionValue :type Boolean) (ElapsedSeconds :type Float%20%28double-precision%29) (TriggeredSeconds :type Float%20%28double-precision%29) (InputAction :type Input%20Action%20Object%20Reference :default "/Game/real/Inputs/IA_Aim.IA_Aim"))
  (bind _as_bp_character (Variables|Default|GetAs%20BP%20Character))
  (bind _returnvalue (Transformation|GetActorLocation _as_bp_character))
  (:Triggered
    (Variables|Default|SetAiming true)
    (Collision|LineTraceByChannel _returnvalue (+ _returnvalue (* (Transformation|GetActorForwardVector _as_bp_character) 6e+02)) "TraceTypeQuery1" false 0 "ForOneFrame"))
  (:Completed
    (Variables|Default|SetAiming false)))

(event Input|EnhancedActionEvents|EnhancedInputActionIA_Rotate
  (params (ActionValue :type Vector :default "0, 0, 0") (ElapsedSeconds :type Float%20%28double-precision%29) (TriggeredSeconds :type Float%20%28double-precision%29) (InputAction :type Input%20Action%20Object%20Reference :default "/Game/real/Inputs/IA_Rotate.IA_Rotate")))

(event EventBeginPlay
  (bind _asbp_character (Utilities|Casting|CastToBP_Character (Game|Player|GetPlayerPawn 0))
    (:then
      (Variables|Default|SetAs%20BP%20Character _asbp_character)
      (Input|AddMappingContext (PlayerController|LocalPlayerSubsystems|GetEnhancedInputLocalPlayerSubsystem self) "/Game/real/Inputs/MC_Example.MC_Example" 0 "(bIgnoreAllPressedKeysUntilRelease=True,bForceImmediately=False,bNotifyUserSettings=False)")
      (Variables|/Script/Engine.PlayerController|SetbShowMouseCursor (Game|GetPlayerController 0) true))
    (:CastFailed
      (Development|PrintString "Character Cast Failed"))))

(event EventTick
  (params (DeltaSeconds :type Float%20%28single-precision%29)))

(fn ConstructionScript)